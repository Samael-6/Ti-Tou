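; BP_Woman is a seated female character who opens a dialogue widget on BeginPlay and idles in a looping sitting animation.
; Dialogue rows come from DT_DialogueFemme by numeric index, filling the widget's text and hiding empty choices; NextDialogue jumps rows.
; Positive and negative expression functions step through clamped material arrays on the mesh.
; Animation plays a random clip, delays by a separately randomized clip's length, then resumes idle.
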(event Custom|StartDialogue
  (bind _returnvalue (UserInterface|CreateWidget "/Game/TieTou/Blueprints/Widget/WBP_Dialogues.WBP_Dialogues_C"))
  (bind _output_get (Variables|Default|SetWBP_Dialogues _returnvalue))
  (Variables|/Game/TieTou/Blueprints/Widget/WBP_Dialogues.WBP_Dialogues_C|SetBP_Woman _output_get self)
  (UserInterface|Viewport|AddtoViewport _output_get 0)
  (CallFunction|GetCurrentRow))

(event Custom|Animation
  (bind _returnvalue (Math|Random|RandomIntegerinRange 0 4))
  (bind _animations (Variables|Default|GetAnimations))
  (bind _output (Utilities|Array|Get(acopy) _animations _returnvalue))
  (Components|Animation|PlayAnimation (Variables|Character|GetMesh) _output false)
  (Utilities|FlowControl|Delay (Animation|GetPlayLength _output))
  (Components|Animation|PlayAnimation (Variables|Character|GetMesh) "/Game/TieTou/Assets/LA_GADJI/ANIMATION_GADJI/Sitting_Idle_Anim.Sitting_Idle_Anim" true))

(event EventBeginPlay
  (Variables|Default|SetDT_Dialogue "/Game/TieTou/Structure/DT_DialogueFemme.DT_DialogueFemme")
  (CallFunction|StartDialogue)
  (Components|Animation|PlayAnimation (Variables|Character|GetMesh) "/Game/TieTou/Assets/LA_GADJI/ANIMATION_GADJI/Sitting_Idle_Anim.Sitting_Idle_Anim" true))

(fn ConstructionScript)

(fn NextDialogue
  (params (NewIndex :type Integer))
  (Variables|Default|SetCurrentIndexRow NewIndex)
  (CallFunction|GetCurrentRow))

(fn GetCurrentRow
  (bind _returnvalue (Utilities|GetDataTableRow (Variables|Default|GetDT_Dialogue) (Utilities|String|StringToName (Utilities|String|ToString(Integer) (Variables|Default|GetCurrentIndexRow))))
    (:then
      (Variables|Default|SetCurrentRow _returnvalue)
      (CallFunction|SetWidgetValue))))

(fn SetWidgetValue
  (bind _wbp_dialogues (Variables|Default|GetWBP_Dialogues))
  (bind _currentrow (Variables|Default|GetCurrentRow))
  (bind _wbp_dialogues_2 (Variables|Default|GetWBP_Dialogues))
  (bind _wbp_dialogues_3 (Variables|Default|GetWBP_Dialogues))
  (bind _wbp_dialogues_4 (Variables|Default|GetWBP_Dialogues))
  (bind (_name _nextrow _timevalue _dialogue _choice1 _choice2 _choice3) (Utilities|Struct|BreakST_Dialogues _currentrow))
  (bind _choice_2 (Variables|/Game/TieTou/Blueprints/Widget/WBP_Dialogues.WBP_Dialogues_C|GetChoice_2 _wbp_dialogues_3))
  (bind _choice_3 (Variables|/Game/TieTou/Blueprints/Widget/WBP_Dialogues.WBP_Dialogues_C|GetChoice_3 _wbp_dialogues_4))
  (bind _choice_1 (Variables|/Game/TieTou/Blueprints/Widget/WBP_Dialogues.WBP_Dialogues_C|GetChoice_1 _wbp_dialogues_2))
  (Variables|/Script/UMG.TextBlock|SetText (Variables|/Game/TieTou/Blueprints/Widget/WBP_Dialogues.WBP_Dialogues_C|GetName _wbp_dialogues) _name)
  (Variables|/Script/UMG.TextBlock|SetText (Variables|/Game/TieTou/Blueprints/Widget/WBP_Dialogues.WBP_Dialogues_C|GetDialogue _wbp_dialogues) _dialogue)
  (Variables|/Script/UMG.TextBlock|SetText (Variables|/Game/TieTou/Blueprints/Widget/WBP_Dialogues.WBP_Dialogues_C|GetTChoice1 _wbp_dialogues) _choice1)
  (Variables|/Script/UMG.TextBlock|SetText (Variables|/Game/TieTou/Blueprints/Widget/WBP_Dialogues.WBP_Dialogues_C|GetTChoice2 _wbp_dialogues) _choice2)
  (Variables|/Script/UMG.TextBlock|SetText (Variables|/Game/TieTou/Blueprints/Widget/WBP_Dialogues.WBP_Dialogues_C|GetTChoice3 _wbp_dialogues) _choice3)
  (Utilities|FlowControl|Sequence
    (:then_0
      (if (Utilities|Enum|Equal(Enum) _choice1 (Variables|Default|GetTextNull))
        (Variables|/Script/UMG.Widget|SetVisibility _choice_1 "Hidden")
        (else
          (Variables|/Script/UMG.Widget|SetVisibility _choice_1 "Visible"))))
    (:then_1
      (if (Utilities|Enum|Equal(Enum) _choice2 (Variables|Default|GetTextNull))
        (Variables|/Script/UMG.Widget|SetVisibility _choice_2 "Hidden")
        (else
          (Variables|/Script/UMG.Widget|SetVisibility _choice_2 "Visible"))))
    (:then_2
      (if (Utilities|Enum|Equal(Enum) _choice3 (Variables|Default|GetTextNull))
        (Variables|/Script/UMG.Widget|SetVisibility _choice_3 "Hidden")
        (else
          (Variables|/Script/UMG.Widget|SetVisibility _choice_3 "Visible"))))))

(fn ExpressionPositive
  (bind _output_get (Variables|Default|SetIndexPositive (+ (Variables|Default|GetIndexPositive) 1)))
  (Rendering|Material|SetMaterial (Variables|Character|GetMesh) 0 (Utilities|Array|Get(acopy) (Variables|Default|GetPositiveExpression) (Math|Integer|Clamp(Integer) _output_get 0 2))))

(fn ExpressionNegative
  (bind _output_get (Variables|Default|SetIndexNegative (+ (Variables|Default|GetIndexNegative) 1)))
  (Rendering|Material|SetMaterial (Variables|Character|GetMesh) 0 (Utilities|Array|Get(acopy) (Variables|Default|GetNegativeExpression) (Math|Integer|Clamp(Integer) _output_get 0 4))))