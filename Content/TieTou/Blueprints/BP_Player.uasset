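; BP_Player is a player Blueprint that opens the main WBP_Menu and flies its camera along a spline.
; BeginPlay shows the mouse cursor, then creates the menu widget and passes it a reference to itself.
; AnimationStart plays the MoveForward timeline at a rate of 1/Duration, moving the camera by fraction of spline length without changing its rotation.
; Completion only prints a debug string.
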(event Custom|AnimationStart
  (bind _spline (Variables|Default|GetSpline))
  (Components|Timeline|SetPlayRate (Variables|Default|GetMoveForward) (/ 1.0 (Variables|Default|GetDuration)))
  (bind _percentage (Timeline|MoveForward PlayFromStart)
    (:Update
      (Transformation|SetWorldLocation (Variables|Default|GetCamera) (Spline|GetLocationatDistanceAlongSpline _spline (* _percentage (Spline|GetSplineLength _spline)) "World") false false))
    (:Finished
      (Development|PrintString "Hello"))))

(event EventBeginPlay
  (Variables|/Script/Engine.PlayerController|SetbShowMouseCursor (Game|GetPlayerController 0) true)
  (bind _returnvalue (UserInterface|CreateWidget "/Game/TieTou/Blueprints/Widget/WBP_Menu.WBP_Menu_C"))
  (Variables|/Game/TieTou/Blueprints/Widget/WBP_Menu.WBP_Menu_C|SetBP_Player _returnvalue self)
  (UserInterface|Viewport|AddtoViewport _returnvalue 0))

(fn ConstructionScript)